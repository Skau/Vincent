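; Game mode Blueprint that picks the player's spawn point based on the teleporter they used.
; Its ChoosePlayerStart override scans every PlayerStart, matching each tag against the last map stored in CustomGameInstance.
; A matching start takes priority, with a start tagged Default or None as the fallback.
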(fn ConstructionScript)

(fn ChoosePlayerStart
  (params (Player :type Controller%20Object%20Reference))
  ;[1 1 1] Custom logic for choosing playerstart depending on what teleporter was used
  (bind _outactors (Actor|GetAllActorsOfClass "/Script/Engine.PlayerStart"))
  (for _array_element _outactors
    (Utilities|FlowControl|Sequence
      (:then_0
        (if (or (Utilities|Name|Equal(Name) (Variables|/Script/Engine.PlayerStart|GetPlayerStartTag _array_element) "Default") (Utilities|Name|Equal(Name) "None" (Variables|/Script/Engine.PlayerStart|GetPlayerStartTag _array_element)))
          (Variables|Default|SetDefaultStart _array_element)))
      (:then_1
        (if (Utilities|Name|Equal(Name) (Variables|/Script/Engine.PlayerStart|GetPlayerStartTag _array_element) (Class|CustomGameInstance|GetLastMap (.AsCustom%20Game%20Instance (Utilities|Casting|CastToCustomGameInstance (Game|GetGameInstance)))))
          (Variables|Default|SetCustomStart _array_element)))))
  (Utilities|IsValid (Variables|Default|GetCustomStart)
    (:Is%20Valid
      (return (Variables|Default|GetCustomStart)))
    (:Is%20Not%20Valid
      (Utilities|IsValid (Variables|Default|GetDefaultStart)
        (:Is%20Valid
          (return (Variables|Default|GetDefaultStart)))))))