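; Enemy character that draws its vision cone as a procedural mesh on a flat horizontal plane.
; Each tick it runs the VisionCone EQS query with all matching results, then converts the returned locations into actor-relative vertices.
; A triangle fan from the center vertex is built into pre-sized arrays and turned into a mesh section, with a material applied and world rotation zeroed so the cone ignores actor rotation.
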(event Custom|MakeMyCone
  (params (QueryInstance :type Env%20Query%20Instance%20Blueprint%20Wrapper%20Object%20Reference) (QueryStatus :type EEnvQueryStatus%20Enum :default "Processing"))
  (bind _output_get (Variables|Default|SetSightPoints (Class|EnvQueryInstanceBlueprintWrapper|GetResultsasLocations QueryInstance)))
  (bind (_vertices _triangles) (CallFunction|ConvertSightPointstoVertices _output_get))
  (CallFunction|MaketheCone _vertices _triangles))

(event EventTick
  (params (DeltaSeconds :type Float%20%28single-precision%29))
  (bind _returnvalue (AI|EQS|RunEQSQuery "/Game/Blueprints/AI/VisionCone.VisionCone" self "AllMatching"))
  (EventDispatchers|BindEventtoOnQueryFinishedEvent _returnvalue (delegate Custom|MakeMyCone)))

(event EventBeginPlay
  (bind _vertices (Variables|Default|GetVertices))
  (Utilities|Array|Resize _vertices 51)
  (Utilities|Array|Resize (Variables|Default|GetTriangles) (* (Utilities|Array|Length _vertices) 3)))

(fn ConstructionScript)

(fn MaketheCone
  (params (Vertices :type Array%20of%20Vectors) (Triangles :type Array%20of%20Integers))
  (bind _procmesh (Variables|Default|GetProcMesh))
  (Class|ProceduralMeshComponent|CreateMeshSectionLinearColor _procmesh 0 Vertices Triangles 0 0 0 0 false)
  (Rendering|Material|SetMaterial _procmesh 0 "/Game/Meshes/Coal_Roller/Materials/blinn6.blinn6")
  (Transformation|SetWorldRotation _procmesh "0, 0, 0" false false))

(fn ConvertSightPointstoVertices
  (params (SightPoints :type Array%20of%20Vectors))
  (bind _returnvalue (Transformation|GetActorLocation))
  (bind (_x _y) (Math|Vector|BreakVector _returnvalue))
  (Utilities|Array|SetArrayElem :TargetArray (Variables|Default|GetVertices))
  (for (_array_element _array_index) SightPoints
    (Utilities|Array|SetArrayElem (Variables|Default|GetVertices) (+ _array_index 1) (Math|Vector|MakeVector (- (.X (Math|Vector|BreakVector _array_element)) _x) (- (.Y (Math|Vector|BreakVector _array_element)) _y) 0.0)))
  (for _index (range 0 (Utilities|Array|LastIndex (Variables|Default|GetVertices)))
    (Utilities|Array|SetArrayElem (Variables|Default|GetTriangles) (* _index 3) 0)
    (Utilities|Array|SetArrayElem (Variables|Default|GetTriangles) (+ (* _index 3) 1) (+ _index 1))
    (Utilities|Array|SetArrayElem (Variables|Default|GetTriangles) (+ (+ (* _index 3) 1) 1) (+ (+ _index 1) 1)))
  (return (Variables|Default|GetVertices) (Variables|Default|GetTriangles)))