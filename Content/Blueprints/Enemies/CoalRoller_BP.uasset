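; Coal Roller enemy Blueprint that handles charge smoke, knockback, facing and a death sound.
; Events toggle the smoke effect for charge build-up, and destruction plays an explosion sound at its location.
; Knockback runs a timeline that sweeps the root opposite the damage causer's forward vector, then resets its knockback state.
; LookAtTarget turns it toward a target but copies the target's pitch.
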(event Custom|ChargeSmokeEnd
  ;[1 1 1] For smoke effect on charge build-up
  (Components|Activation|SetActive (Variables|Default|GetChargeSmoke) false false))

(event Custom|ChargeSmokeBegin
  ;[1 1 1] For smoke effect on charge build-up
  (Components|Activation|SetActive (Variables|Default|GetChargeSmoke) true false))

(event EventKnockback
  (params (DamageCauser :type Actor%20Object%20Reference))
  ;[1 1 1] Knockback event
  (Variables|Default|SetIsBeingKnockbacked true)
  (bind _offset (Timeline|KnockbackTimeline PlayFromStart)
    (:Update
      (Transformation|AddWorldOffset (Variables|Transformation|GetRootComponent) (* (* (* (Transformation|GetActorForwardVector DamageCauser) -1.0) _offset) (Utilities|Time|GetWorldDeltaSeconds)) true false))
    (:Finished
      (Class|CoalRoller|ResetHasBeenKnockedBack)
      (Variables|Default|SetIsBeingKnockbacked false))))

(event EventDestroyed
  (Audio|PlaySoundatLocation "/Game/Audio/SFX/explode.explode" (Transformation|GetActorLocation)))

(event EventBeginPlay
  (Components|Activation|Deactivate (Variables|Default|GetChargeSmoke)))

(fn ConstructionScript)

(fn LookatTarget
  (params (TargetActor :type Actor%20Object%20Reference))
  (bind _returnvalue (Transformation|GetActorLocation TargetActor))
  (bind _returnvalue_2 (Transformation|GetActorLocation))
  (bind _returnvalue_3 (Math|Rotator|FindLookatRotation _returnvalue_2 _returnvalue))
  (Transformation|SetActorRotation (Math|Rotator|MakeRotator (.roll _returnvalue_3) (.pitch (Transformation|GetActorRotation TargetActor)) (.yaw _returnvalue_3))))