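; Destructible wall actor that, once fractured, tells its linked spawnpoint to stop spawning bombwalkers.
; On fracture it restores its original material, notifies the spawnpoint and destroys itself after a short delay.
; SetMaterialTransparent swaps in a see-through material, while Tick restores the original every frame, so transparency lasts only until the next tick.
; Both material setters skip the swap when that material is already applied.
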(event Custom|OnFracture
  (params (HitPoint :type Vector%20%28by%20ref%29) (HitDirection :type Vector%20%28by%20ref%29))
  ;[1 1 1] On destroyed wall, tell spawnpoint to stop spawning bombwalkers
  (CallFunction|SetMaterialOriginal)
  (Class|SpawnPoint|SetWallIsFractured (Variables|Default|GetSpawnpointRef))
  (Utilities|FlowControl|Delay 2.0)
  (Actor|DestroyActor))

(event EventBeginPlay
  ;[1 1 1] On destroyed wall, tell spawnpoint to stop spawning bombwalkers
  (EventDispatchers|BindEventtoOnActorFracture (delegate Custom|OnFracture)))

(event EventTick
  (params (DeltaSeconds :type Float%20%28single-precision%29))
  (CallFunction|SetMaterialOriginal))

(event EventSetMaterialOriginal
  (if (not (== (Rendering|Material|GetMaterial (Variables|Default|GetDestructibleComponent) 0) (Variables|Default|GetOriginalMaterial)))
    (Rendering|Material|SetMaterial (Variables|Default|GetDestructibleComponent) 0 (Variables|Default|GetOriginalMaterial))))

(event EventSetMaterialTransparent
  (if (not (== (Rendering|Material|GetMaterial (Variables|Default|GetDestructibleComponent) 0) (Variables|Default|GetTransparentMaterial)))
    (Rendering|Material|SetMaterial (Variables|Default|GetDestructibleComponent) 0 (Variables|Default|GetTransparentMaterial))))

(fn ConstructionScript)