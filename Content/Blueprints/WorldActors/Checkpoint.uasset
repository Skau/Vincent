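; Checkpoint world actor that sets the player's respawn point when overlapped and lets the hammer be picked up nearby.
; The first player overlap passes its location, offset along X, to PlayerCharacter_BP and flags itself as current spawn; later overlaps only print a message.
; Begin and end overlap also toggle the player's BIsCloseEnough flag, which enables hammer pickup.
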(event Collision|EventActorBeginOverlap
  (params (OtherActor :type Actor%20Object%20Reference))
  ;[1 1 1] Comment
  (Utilities|FlowControl|Sequence
    (:then_0
      (if (Variables|Default|GetIsCurrentSpawn)
        ;[1 1 1] MOVE TO HUD
        (Development|PrintString "Already a checkpoint!")
        (else
          (Development|PrintString "Checkpoint!")
          (bind _asplayer_character_bp (Utilities|Casting|CastToPlayerCharacter_BP OtherActor))
          (Class|PlayerCharacter|SetNewSpawnPoint _asplayer_character_bp (+ (Transformation|GetActorLocation) "-100.000000, 0, 0"))
          (Variables|Default|SetIsCurrentSpawn true))))
    (:then_1
      ;[1 1 1] Makes hammer pickupable
      (bind _asplayer_character_bp_2 (Utilities|Casting|CastToPlayerCharacter_BP OtherActor))
      (Class|PlayerCharacter|SetBIsCloseEnough _asplayer_character_bp_2 true))))

(event Collision|EventActorEndOverlap
  (params (OtherActor :type Actor%20Object%20Reference))
  ;[1 1 1] Makes hammer pickupable
  (bind _asplayer_character_bp (Utilities|Casting|CastToPlayerCharacter_BP OtherActor))
  (Class|PlayerCharacter|SetBIsCloseEnough _asplayer_character_bp false))

(fn ConstructionScript)