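; Wall actor whose static mesh can switch between an original material and a transparent one.
; Tick restores the original material every frame, so transparency set through SetMaterialTransparent lasts only until the wall's next Tick unless it is called again.
; Both setter events check the material in slot 0 first and assign only when it differs.
; No caller of the transparent event appears in this Blueprint.
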(event EventSetMaterialTransparent
  (if (not (== (Rendering|Material|GetMaterial (Variables|Default|GetStaticMesh) 0) (Variables|Default|GetTransparentMaterial)))
    (Rendering|Material|SetMaterial (Variables|Default|GetStaticMesh) 0 (Variables|Default|GetTransparentMaterial))))

(event EventSetMaterialOriginal
  (if (not (== (Rendering|Material|GetMaterial (Variables|Default|GetStaticMesh) 0) (Variables|Default|GetOriginalMaterial)))
    (Rendering|Material|SetMaterial (Variables|Default|GetStaticMesh) 0 (Variables|Default|GetOriginalMaterial))))

(event EventTick
  (params (DeltaSeconds :type Float%20%28single-precision%29))
  (CallFunction|SetMaterialOriginal))

(fn ConstructionScript)