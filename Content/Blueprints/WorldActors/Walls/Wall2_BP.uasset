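; Wall actor that switches its static mesh to a transparent material while it blocks the player's line trace.
; The player calls interface events that set either the original or transparent material on slot 0, skipping the change if that material is already applied.
; Tick attempts to restore the original material every frame, relying on the player to override it while the wall is blocking.
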(event EventSetMaterialTransparent
  ;[1 1 1] Interface functions called by player on linetrace block
  (if (not (== (Rendering|Material|GetMaterial (Variables|Default|GetStaticMesh) 0) (Variables|Default|GetTransparentMaterial)))
    (Rendering|Material|SetMaterial (Variables|Default|GetStaticMesh) 0 (Variables|Default|GetTransparentMaterial))))

(event EventSetMaterialOriginal
  ;[1 1 1] Interface functions called by player on linetrace block
  (if (not (== (Rendering|Material|GetMaterial (Variables|Default|GetStaticMesh) 0) (Variables|Default|GetOriginalMaterial)))
    (Rendering|Material|SetMaterial (Variables|Default|GetStaticMesh) 0 (Variables|Default|GetOriginalMaterial))))

(event EventTick
  (params (DeltaSeconds :type Float%20%28single-precision%29))
  ;[1 1 1] Trys to set material back to original (overriden by player if blocking)
  (CallFunction|SetMaterialOriginal))

(fn ConstructionScript)