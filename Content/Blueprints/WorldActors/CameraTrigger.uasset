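; CameraTrigger is a world actor that plays a level sequence when the player character enters its overlap.
; On overlap with PlayerCharacter_BP it creates a level sequence player from the assigned sequence and passes it to CustomPlayerController_BP to play.
; A HasPlayed flag makes it fire only once, and later overlaps just print a debug message.
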(event Collision|EventActorBeginOverlap
  (params (OtherActor :type Actor%20Object%20Reference))
  (bind (_asplayer_character_bp _bsuccess) (Utilities|Casting|CastToPlayerCharacter_BP OtherActor))
  (if (Variables|Default|GetHasPlayed)
    (Development|PrintString "Sequence has already played once!")
    (elif _bsuccess
      (bind _returnvalue (Sequencer|Player|CreateLevelSequencePlayer (Variables|Default|GetLevelSequenceToPlay)))
      (Default|PlaySequence (.AsCustom%20Player%20Controller%20BP (Utilities|Casting|CastToCustomPlayerController_BP (Pawn|GetController _asplayer_character_bp))) _returnvalue)
      (Variables|Default|SetHasPlayed true))))

(fn ConstructionScript)