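; Player character Blueprint that adds minimap, damage feedback, knockback and death-screen behavior on top of C++ damage logic.
; On BeginPlay it attaches the level's MiniMapCam to itself, drives its update from Tick, and zooms it between three clamped levels via input.
; Timelines fade a red damage effect and apply swept capsule knockback.
; CreateDeathWidget shows the death UI and pauses the game, while DoJump serves the AnimBP.
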(event Custom|CreateDeathWidget
  (bind _returnvalue (Game|GetPlayerController 0))
  (bind _returnvalue_2 (UserInterface|CreateWidget "/Game/UI/Widgets/DeathWidget.DeathWidget_C" _returnvalue))
  (bind _output_get (Variables|Default|SetDeathWidget _returnvalue_2))
  (UserInterface|Viewport|AddtoViewport _output_get 0)
  (Input|SetInputModeUIOnly _returnvalue _output_get "LockOnCapture")
  (Game|SetGamePaused true))

(event Custom|DoJump
  ;[1 1 1] Called from animbp
  (Character|Jump))

(event Game|Damage|EventAnyDamage
  (params (Damage :type Float%20%28single-precision%29) (DamageType :type Damage%20Type%20Object%20Reference) (InstigatedBy :type Controller%20Object%20Reference) (DamageCauser :type Actor%20Object%20Reference))
  ;[1 1 1] Main damage logic is in c++, this is just here for the red effect on damage taken (Timelines not available in c++)
  (if (not (Class|PlayerCharacter|GetIsDead))
    (bind _blendweight (Timeline|Fade%20BW%20Over%20Time PlayFromStart)
      (:Update
        (Variables|/Script/Engine.PostProcessComponent|SetBlendWeight (Variables|Default|GetDamageTakenFade) _blendweight)))))

(event EventBeginPlay
  ;[1 1 1] Find MiniMapCam and attach to actor
  (Utilities|IsValid (Variables|Default|GetMiniMapCam)
    (:Is%20Not%20Valid
      (bind _outactors (Actor|GetAllActorsOfClass "/Game/MiniMap/MiniMapCam.MiniMapCam_C"))
      (for _array_element _outactors
        (bind _output_get (Variables|Default|SetMiniMapCam _array_element))
        (Transformation|AttachActorToActor _output_get self "None" "KeepRelative" "KeepRelative" "KeepRelative" true)))))

(event EventTick
  (params (DeltaSeconds :type Float%20%28single-precision%29))
  (bind _deathwidget (Variables|Default|GetDeathWidget))
  (bind _minimapcam (Variables|Default|GetMiniMapCam))
  (Variables|Default|SetDeltaSeconds DeltaSeconds)
  (Utilities|FlowControl|Sequence
    (:then_0
      ;[1 1 1] Custom Tick for minimap (So minimap follows PlayerTick)
      (Utilities|IsValid _minimapcam
        (:Is%20Valid
          (Default|OutSideTick _minimapcam))))
    (:then_1
      (Utilities|IsValid _deathwidget
        (:Is%20Valid
          (if (not (Widget|IsVisible _deathwidget))
            (Widget|RemovefromParent _deathwidget)))))))

(event EventKnockback
  (params (EnemyCauser :type Actor%20Object%20Reference) (ActorForwardVector :type Vector :default "0, 0, 0"))
  ;[1 1 1] Knocback event when taking damage
  (bind _offset (Timeline|Offset%20Timeline PlayFromStart)
    (:Update
      (Transformation|AddWorldOffset (Variables|Default|GetCapsuleComponent) (* (* ActorForwardVector _offset) (Variables|Default|GetDeltaSeconds)) true false))))

(event Input|ActionEvents|InputActionMiniMapCamZoomIn
  (params (Key :type Key%20Structure))
  ;[1 1 1] Zooming logic for MiniMap (3 levels of zoom so you can't zoom in or out forever)
  (:Pressed
    (if (> (Variables|Default|GetZoomLevel) 1)
      (Transformation|AddLocalOffset (Variables|/Script/Engine.SceneCapture2D|GetCaptureComponent2D (Variables|Default|GetMiniMapCam)) "1500.000000,0.000000,0.000000" false false)
      (Math|Integer|DecrementInt (Variables|Default|GetZoomLevel)))))

(event Input|ActionEvents|InputActionMiniMapCamZoomOut
  (params (Key :type Key%20Structure))
  ;[1 1 1] Zooming logic for MiniMap (3 levels of zoom so you can't zoom in or out forever)
  (:Pressed
    (if (< (Variables|Default|GetZoomLevel) 3)
      (Transformation|AddLocalOffset (Variables|/Script/Engine.SceneCapture2D|GetCaptureComponent2D (Variables|Default|GetMiniMapCam)) "-1500.000000, 0, 0" false false)
      (Math|Integer|IncrementInt (Variables|Default|GetZoomLevel)))))

(fn ConstructionScript)