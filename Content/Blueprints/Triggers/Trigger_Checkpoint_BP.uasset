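; Checkpoint trigger Blueprint that shows on-screen feedback for a checkpoint prompt and for a checkpoint being taken.
; Two events, called from C++, each create their widget for player 0 and add it to the viewport.
; A separate timeline per event animates the widget's text opacity, then removes the widget and clears the widget-playing flag when finished.
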(event EventCreateCheckpointPromptWidget
  ;[1 1 1] Events called from c++ for widget creation
  (bind _returnvalue (UserInterface|CreateWidget "/Game/UI/Widgets/CheckpointPrompt.CheckpointPrompt_C" (Game|GetPlayerController 0)))
  (UserInterface|Viewport|AddtoViewport _returnvalue 0)
  (bind _opacity (Timeline|SetOpacity2 PlayFromStart)
    (:Update
      (Class|TextBlock|SetOpacity (Variables|/Game/UI/Widgets/CheckpointPrompt.CheckpointPrompt_C|GetText _returnvalue) _opacity))
    (:Finished
      (Widget|RemovefromParent _returnvalue)
      (Class|TriggerCheckpoint|SetIsWidgetPlaying false))))

(event EventCreateCheckpointTakenWidget
  ;[1 1 1] Events called from c++ for widget creation
  (bind _returnvalue (UserInterface|CreateWidget "/Game/UI/Widgets/CheckpointTaken.CheckpointTaken_C" (Game|GetPlayerController 0)))
  (UserInterface|Viewport|AddtoViewport _returnvalue 0)
  (bind _opacity (Timeline|SetOpacity PlayFromStart)
    (:Update
      (Class|TextBlock|SetOpacity (Variables|/Game/UI/Widgets/CheckpointTaken.CheckpointTaken_C|GetText _returnvalue) _opacity))
    (:Finished
      (Widget|RemovefromParent _returnvalue)
      (Class|TriggerCheckpoint|SetIsWidgetPlaying false))))

(fn ConstructionScript)