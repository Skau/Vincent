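; Trigger Blueprint for a door teleporter, with events called from C++ during teleporting.
; A timeline animates the door mesh yaw to close it, then teleports the player if they are inside when it finishes.
; Opening reverses that timeline, from the end for the first opening.
; A separate event shows the HUD loading widget, waits briefly, then opens the requested map by name.
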(event EventOpenNewMapwithLoading
  (params (MapToLoad :type Name%20%28by%20ref%29 :default "None"))
  ;[1 1 1] Events called from C++ when teleporting
  (Default|LoadWidgetin (.AsPlayer%20HUD (Utilities|Casting|CastToPlayerHUD (HUD|GetHUD (Game|GetPlayerController 0)))))
  (Utilities|FlowControl|Delay 2.0)
  (Game|OpenLevel(byName) MapToLoad))

(event EventOpenDoor
  ;[1 1 1] Events called from C++ when teleporting
  (bind _dooryawrotation (Timeline|TL_CloseDoor Reverse)
    (:Update
      (Transformation|SetRelativeRotation (Class|TriggerTeleporter|GetDoorMesh) (Math|Rotator|MakeRotator 0.0 0.0 _dooryawrotation) false false))
    (:Finished
      (if (Variables|Default|GetbPlayerIsInside)
        (Class|TriggerTeleporter|TeleportPlayer)))))

(event EventOpenDoorFirstTime
  ;[1 1 1] Events called from C++ when teleporting
  (bind _dooryawrotation (Timeline|TL_CloseDoor ReverseFromEnd)
    (:Update
      (Transformation|SetRelativeRotation (Class|TriggerTeleporter|GetDoorMesh) (Math|Rotator|MakeRotator 0.0 0.0 _dooryawrotation) false false))
    (:Finished
      (if (Variables|Default|GetbPlayerIsInside)
        (Class|TriggerTeleporter|TeleportPlayer)))))

(event EventCloseDoor
  ;[1 1 1] Events called from C++ when teleporting
  (bind _dooryawrotation (Timeline|TL_CloseDoor Play)
    (:Update
      (Transformation|SetRelativeRotation (Class|TriggerTeleporter|GetDoorMesh) (Math|Rotator|MakeRotator 0.0 0.0 _dooryawrotation) false false))
    (:Finished
      (if (Variables|Default|GetbPlayerIsInside)
        (Class|TriggerTeleporter|TeleportPlayer)))))

(fn ConstructionScript)