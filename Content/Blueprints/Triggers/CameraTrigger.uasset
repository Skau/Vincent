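; CameraTrigger is a trigger actor that starts a level sequence when the player character walks through it.
; On overlap with PlayerCharacter_BP, it creates a player for LevelSequenceToPlay and passes it to CharacterPlayerController_BP's PlaySequence.
; A HasPlayed flag limits it to one playback, with later overlaps only printing a message.
; The graph notes that sequences are cut from the final game, with the logic kept for possible reuse.
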(event Collision|EventActorBeginOverlap
  (params (OtherActor :type Actor%20Object%20Reference))
  (bind (_asplayer_character_bp _bsuccess) (Utilities|Casting|CastToPlayerCharacter_BP OtherActor))
  ;[1 1 1] Triggers sequence when walked through. Sequences are not part of the final game, but all logic is still available if we want to implement them back later
  (if _bsuccess
    (if (Variables|Default|GetHasPlayed)
      (Development|PrintString "Sequence has already played once!")
      (else
        (bind _returnvalue (Sequencer|Player|CreateLevelSequencePlayer (Variables|Default|GetLevelSequenceToPlay)))
        (Default|PlaySequence (.AsCharacter%20Player%20Controller%20BP (Utilities|Casting|CastToCharacterPlayerController_BP (Pawn|GetController _asplayer_character_bp))) _returnvalue)
        (Variables|Default|SetHasPlayed true)))))

(fn ConstructionScript)