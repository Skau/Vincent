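; AI controller that drives CoalRoller and BombRoller enemies with knowledge of the player's location.
; Every Tick it sets up the shared blackboard and, if player 0's character is valid, writes that location to a vector key.
; It then runs the CoalRoller behavior tree for a CoalRoller pawn, or the BombRoller tree for anything else.
; Blackboard setup and tree start both happen in Tick rather than on possession.
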(event EventTick
  (params (DeltaSeconds :type Float%20%28single-precision%29))
  (bind _returnvalue (Game|GetPlayerCharacter 0))
  (bind _returnvalue_2 (Game|GetPlayerCharacter 0))
  (bind _asplayer_character_bp (Utilities|Casting|CastToPlayerCharacter_BP _returnvalue))
  (bind _asplayer_character_bp_2 (Utilities|Casting|CastToPlayerCharacter_BP _returnvalue_2))
  (if (.bSuccess (Utilities|Casting|CastToCoalRoller_BP (Pawn|GetControlledPawn self)))
    ;[1 1 1] CoalRoller AI
    (bind _blackboardcomponent (Class|AIController|UseBlackboard "/Game/Blueprints/AI/AIBlackBoard.AIBlackBoard"))
    (Utilities|IsValid _asplayer_character_bp_2
      (:Is%20Valid
        (AI|Components|Blackboard|SetValueasVector _blackboardcomponent (Variables|Default|GetKeyName) (Transformation|GetActorLocation _asplayer_character_bp_2))
        (AI|RunBehaviorTree "/Game/Blueprints/AI/AIBT_CoalRoller.AIBT_CoalRoller")))
    (else
      ;[1 1 1] BombRoller AI
      (bind _blackboardcomponent_2 (Class|AIController|UseBlackboard "/Game/Blueprints/AI/AIBlackBoard.AIBlackBoard"))
      (Utilities|IsValid _asplayer_character_bp
        (:Is%20Valid
          (AI|Components|Blackboard|SetValueasVector _blackboardcomponent_2 (Variables|Default|GetKeyName) (Transformation|GetActorLocation _asplayer_character_bp))
          (AI|RunBehaviorTree "/Game/Blueprints/AI/AIBT_BombRoller.AIBT_BombRoller"))))))

(fn ConstructionScript)