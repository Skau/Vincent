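; Player controller Blueprint that plays level sequences and lets the player skip them with the SkipSequence input.
; PlaySequence stores and starts the given sequence player, and the input stops it while it is playing.
; Tick polls that player to toggle the cursor and playing flag, adding a new skip-text widget every frame during playback and removing them all afterwards.
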(event Custom|PlaySequence
  (params (LevelSequencePlayer :type Level%20Sequence%20Player%20Object%20Reference))
  ;[1 1 1] PlaySequence event
  (bind _output_get (Variables|Default|SetLevelSequencePlayer LevelSequencePlayer))
  (Sequencer|Player|Play _output_get :!class /Script/MovieScene.MovieSceneSequencePlayer))

(event EventTick
  (params (DeltaSeconds :type Float%20%28single-precision%29))
  (bind _levelsequenceplayer (Variables|Default|GetLevelSequencePlayer))
  ;[1 1 1] Skip sequence text. Doing this here, because the HUD is hidden during sequence (And we have to remove/show cursor anyways)
  (Utilities|IsValid _levelsequenceplayer
    (:Is%20Valid
      (if (Audio|Components|Audio|IsPlaying _levelsequenceplayer)
        (Variables|Default|SetbShowMouseCursor false)
        (Class|CharacterPlayerController|SetIsSequencePlaying true)
        (bind _returnvalue (UserInterface|CreateWidget "/Game/UI/Widgets/SkipSequenceText.SkipSequenceText_C"))
        (UserInterface|Viewport|AddtoViewport _returnvalue 0)
        (else
          (Variables|Default|SetbShowMouseCursor true)
          (Class|CharacterPlayerController|SetIsSequencePlaying false)
          (bind _foundwidgets (Widget|GetAllWidgetsOfClass "/Game/UI/Widgets/SkipSequenceText.SkipSequenceText_C" true))
          (Widget|RemovefromParent _foundwidgets))))))

(event Input|ActionEvents|InputActionSkipSequence
  (params (Key :type Key%20Structure))
  (bind _levelsequenceplayer (Variables|Default|GetLevelSequencePlayer))
  ;[1 1 1] Inputlogic to skip sequence
  (:Pressed
    (Utilities|IsValid _levelsequenceplayer
      (:Is%20Valid
        (if (Audio|Components|Audio|IsPlaying _levelsequenceplayer)
          (Sequencer|Player|Stop (Variables|Default|GetLevelSequencePlayer) :!class /Script/MovieScene.MovieSceneSequencePlayer))))))

(fn ConstructionScript)