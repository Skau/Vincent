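; Player controller Blueprint that plays level sequences and tracks whether one is currently playing.
; The PlaySequence event stores the given sequence player and starts playback.
; Every tick it polls that player, hiding the mouse cursor and setting the sequence-playing flag during playback, then showing the cursor and clearing the flag whenever it is not playing.
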(event Custom|PlaySequence
  (params (LevelSequencePlayer :type Level%20Sequence%20Player%20Object%20Reference))
  (bind _output_get (Variables|Default|SetLevelSequencePlayer LevelSequencePlayer))
  (Sequencer|Player|Play _output_get :!class /Script/MovieScene.MovieSceneSequencePlayer))

(event EventTick
  (params (DeltaSeconds :type Float%20%28single-precision%29))
  (bind _levelsequenceplayer (Variables|Default|GetLevelSequencePlayer))
  (Utilities|IsValid _levelsequenceplayer
    (:Is%20Valid
      (if (Audio|Components|Audio|IsPlaying _levelsequenceplayer)
        (Variables|Default|SetbShowMouseCursor false)
        (Class|CustomPlayerController|SetIsSequencePlaying true)
        (else
          (Variables|Default|SetbShowMouseCursor true)
          (Class|CustomPlayerController|SetIsSequencePlaying false))))))

(fn ConstructionScript)